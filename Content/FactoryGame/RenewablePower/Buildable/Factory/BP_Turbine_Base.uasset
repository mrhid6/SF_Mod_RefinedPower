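; Base buildable for wind and water turbine generators that feeds renewable power into the grid through its power connection.
; Each factory tick sets production by turbine type, with water turbines requiring overlap with a water volume.
; Wind output optionally scales with height and is shared among turbines found by a periodic sphere overlap, dropping to zero at the crowding limit.
; Animation helpers follow connection and enabled state, with crowding slowing the wind animation.
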(event EventBeginPlay
  (CallFunction|GetWindTurbinesinSphere))

(event Collision|EventActorBeginOverlap
  (params (OtherActor :type Actor%20Object%20Reference)))

(event EventFactoryReceiveTick
  (params (deltaTime :type Float%20%28single-precision%29))
  (CallFunction|ToggleTurbineAirAnimation)
  (switch Utilities|FlowControl|Switch|SwitchonEnum_TurbineType (Variables|Default|GetTurbineType)
    (:NewEnumerator0
      (bind _powermw (CallFunction|GetTurbineAirPowerProduction)))
    (:NewEnumerator1
      (bind _powermw_2 (CallFunction|GetTurbineWaterPowerProduction))))
  (Class|FGPowerInfoComponent|SetBaseProduction (Class|FGPowerConnectionComponent|GetPowerInfo (Variables|Generator|GetFGPowerConnection)) (Math|Float|SelectFloat _powermw _powermw_2 (Utilities|Enum|Equal(Enum) (Variables|Default|GetTurbineType) "NewEnumerator0")))
  (if (Utilities|Enum|Equal(Enum) (Variables|Default|GetTurbineType) "NewEnumerator0")
    (Utilities|FlowControl|Delay 1e+01)
    (CallFunction|GetWindTurbinesinSphere)))

(fn ConstructionScript)

(fn CanStartPowerProduction
  (return (Variables|Generator|GetCanStart)))

(fn CanProduce
  (return (Variables|Generator|GetCanStart)))

(fn GetProductionMW
  (return (Math|Float|SelectFloat (Variables|Default|GetBaseProduction) 0.0 (Variables|Default|GetisTurbineEnabled))))

(fn ToggleTurbineAirAnimation
  (params (SkelMesh :type Skeletal%20Mesh%20Component%20Object%20Reference) (NewAnimToPlay :type Animation%20Asset%20Object%20Reference))
  (bind _returnvalue (Audio|Components|Audio|IsPlaying SkelMesh))
  (Components|Timeline|SetPlayRate SkelMesh (Math|Float|Clamp(Float) (* (/ 1.0 (Math|Conversions|ToFloat(Integer) (Variables|Default|GetMaxTurbinesInArea))) (Math|Conversions|ToFloat(Integer) (- (Variables|Default|GetMaxTurbinesInArea) (Variables|Default|GetTurbinesInArea))))))
  (if (and (Math|Conversions|ToBoolean(Integer) (Class|FGCircuitConnectionComponent|IsConnected (Variables|Generator|GetFGPowerConnection))) (Variables|Default|GetisTurbineEnabled))
    (if (not _returnvalue)
      (Components|Animation|PlayAnimation SkelMesh NewAnimToPlay true))
    (elif _returnvalue
      (Audio|Components|Audio|Stop SkelMesh))))

(fn GetProductionMWHeight
  (bind _snap (Variables|Default|GetSnap))
  (bind _baseproduction (Variables|Default|GetBaseProduction))
  (bind _returnvalue (Transformation|GetWorldLocation _snap))
  (bind _z (Math|Vector|BreakVector _returnvalue))
  (bind _returnvalue_2 (/ _z 8e+02))
  (return (Math|Float|SelectFloat (Math|Float|Clamp(Float) (+ (* (- (Math|Float|SelectFloat (Variables|Default|GetBaseProduction) _returnvalue_2 (< _returnvalue_2 7.0)) _baseproduction) (Variables|Default|GetProductionHeightModifier)) _baseproduction) 1e+01 3e+01) 0.0 (Variables|Default|GetisTurbineEnabled))))

(fn GetTurbineAirPowerProduction
  (if (>= (Variables|Default|GetTurbinesInArea) (Variables|Default|GetMaxTurbinesInArea))
    (return 0.0)
    (else
      (if (Variables|Default|GetApplyHeightMultiplier)
        (bind _returnvalue (CallFunction|GetProductionMWHeight))
        (else
          (bind _returnvalue_2 (CallFunction|GetProductionMW))))
      (return (Math|Float|SelectFloat 0.0 (Math|Float|SelectFloat (Math|Float|Clamp(Float) (/ _returnvalue (Math|Conversions|ToFloat(Integer) (+ (Variables|Default|GetTurbinesInArea) 1))) 0.0 _returnvalue) (Math|Float|Clamp(Float) (/ _returnvalue_2 (Math|Conversions|ToFloat(Integer) (+ (Variables|Default|GetTurbinesInArea) 1))) 0.0 _returnvalue_2) (Variables|Default|GetApplyHeightMultiplier)) (>= (Variables|Default|GetTurbinesInArea) (Variables|Default|GetMaxTurbinesInArea)))))))

(fn GetTurbineWaterPowerProduction
  (bind _return_value (CallFunction|CheckTurbineinWater))
  (return (Math|Float|SelectFloat (Variables|Default|GetBaseProduction) 0.0 (and (Variables|Default|GetisTurbineEnabled) _return_value))))

(fn CheckTurbineinWater
  (bind _outactors (Actor|GetAllActorsOfClass "/Script/FactoryGame.FGWaterVolume"))
  (bind _array_element (Utilities|Array|ForEachLoopwithBreak _outactors)
    (:LoopBody
      (if (Collision|IsOverlappingActor (Variables|Default|GetWaterTest) _array_element :!class /Script/Engine.PrimitiveComponent)
        (return (Collision|IsOverlappingActor (Variables|Default|GetWaterTest) _array_element :!class /Script/Engine.PrimitiveComponent) _array_element)))
    (:Completed
      (return (Collision|IsOverlappingActor (Variables|Default|GetWaterTest) _array_element :!class /Script/Engine.PrimitiveComponent) _array_element))))

(fn ToggleTurbineWaterAnimation
  (params (SkelMesh :type Skeletal%20Mesh%20Component%20Object%20Reference) (NewAnimToPlay :type Animation%20Asset%20Object%20Reference))
  (bind _returnvalue (Audio|Components|Audio|IsPlaying SkelMesh))
  (bind _return_value (CallFunction|CheckTurbineinWater))
  (if (Math|Boolean|ANDBoolean _return_value (Math|Conversions|ToBoolean(Integer) (Class|FGCircuitConnectionComponent|IsConnected (Variables|Generator|GetFGPowerConnection))) (Variables|Default|GetisTurbineEnabled))
    (if _returnvalue
      (return)
      (else
        (Components|Animation|PlayAnimation SkelMesh NewAnimToPlay true)))
    (elif _returnvalue
      (Audio|Components|Audio|Stop SkelMesh)
      (else
        (return))))
  (return))

(fn GetWindTurbinesinSphere
  (bind _windturbinetest (Variables|Default|GetWindTurbineTest))
  (Variables|Default|SetTurbinesInArea 0)
  (bind _outactors (Collision|SphereOverlapActors (Transformation|GetWorldLocation _windturbinetest) (Variables|/Script/Engine.SphereComponent|GetSphereRadius _windturbinetest) (Utilities|Array|MakeArray "ObjectTypeQuery1" "ObjectTypeQuery2") "BP_Turbine_Base_C"))
  (for _array_element _outactors
    (bind _asbp_turbine_base (Utilities|Casting|CastToBP_Turbine_Base _array_element))
    (if (!= _asbp_turbine_base self)
      (switch Utilities|FlowControl|Switch|SwitchonEnum_TurbineType (Variables|BP_Turbine_Base_C|GetTurbineType _asbp_turbine_base)
        (:NewEnumerator0
          (bind _result (Math|Integer|IncrementInt (Variables|Default|GetTurbinesInArea))
            (:%20%20
              (Variables|Default|SetTurbinesInArea _result)))))))
  (return (Variables|Default|GetTurbinesInArea)))